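; Game mode for a time control and replay system that spawns the player pawns and controls time.
; On BeginPlay it spawns character and vehicle pawns at tagged actors and caches the spectator pawn.
; It broadcasts time direction through BPI_TimeControlSystem and steps global dilation in half increments, optionally counter-scaling the player pawn and itself.
; It also saves character and vehicle replay data to a slot and loads it back.
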(event `self.ReceiveBeginPlay`
  (`self.SpawnCharacter`)
  (`self.SpawnVehicle`)
  (`self.SpawnSpectator`))

(fn `DecreaseDilation`
  (`self.ModifyTimeDilation` -0.5))

(fn `IncreaseDilation`
  (`self.ModifyTimeDilation` 0.5))

(fn `LoadGame`
  (returns (SaveGameObject :type "SaveGame Object Reference"))
  (bind _returnvalue (`GameplayStatics.LoadGameFromSlot` (`self.SaveSlotName`)))
  (return _returnvalue))

(fn `ModifyTimeDilation`
  (params (TimeDilation :type "Float (double-precision)"))
  (bind _returnvalue (/ 1.0 (`GameplayStatics.GetGlobalTimeDilation`)))
  (`GameplayStatics.SetGlobalTimeDilation` (`KismetMathLibrary.GridSnap_Float` (+ TimeDilation (`GameplayStatics.GetGlobalTimeDilation`)) 0.5))
  (if (not (`self.DilationAffectsPlayers`))
    (set `Actor.CustomTimeDilation` _returnvalue (`GameplayStatics.GetPlayerPawn` 0))
    (set `self.CustomTimeDilation` _returnvalue)))

(fn `SaveGame`
  (params (CharacterReplayData :type "Array of /Game/TimeControlSystem/Blueprints/ReplaySystem/Struct_ReplayDataCharacter Structure") (VehicleReplayData :type "Array of /Game/TimeControlSystem/Blueprints/ReplaySystem/Struct_ReplayDataVehicle Structure"))
  (returns (ReturnValue :type Boolean))
  (`self.SaveGameObject`
    (:`then`
      _)
    (:`else`
      (bind _returnvalue (`GameplayStatics.CreateSaveGameObject` "/Game/TimeControlSystem/Blueprints/ReplaySystem/BP_ReplaySaveGame.BP_ReplaySaveGame_C"))
      (set `self.SaveGameObject` _returnvalue)))
  (set `/Game/TimeControlSystem/Blueprints/ReplaySystem/BP_ReplaySaveGame.CharacterReplayData` (`local.CharacterReplayData`) (`self.SaveGameObject`))
  (set `/Game/TimeControlSystem/Blueprints/ReplaySystem/BP_ReplaySaveGame.VehicleReplayData` (`local.VehicleReplayData`) (`self.SaveGameObject`))
  (bind _returnvalue_2 (`GameplayStatics.SaveGameToSlot` (`self.SaveGameObject`) (`self.SaveSlotName`)))
  (return _returnvalue_2))

(fn `SetTimeDirection`
  (params (TimeDirection :type "/Game/TimeControlSystem/Blueprints/Enum_TimeDirection Enum" :default "NewEnumerator0"))
  (set `self.TimeDirection` TimeDirection)
  (bind _outactors (`GameplayStatics.GetAllActorsWithInterface` "/Game/TimeControlSystem/Blueprints/BPI_TimeControlSystem.BPI_TimeControlSystem_C"))
  (message `/Game/TimeControlSystem/Blueprints/BPI_TimeControlSystem.BPI_SetTimeDirection` _outactors (`self.TimeDirection`)))

(fn `SpawnCharacter`
  (bind _outactors (`GameplayStatics.GetAllActorsWithTag` "MannequinPawn"))
  (bind _returnvalue (`|SpawnActorFromClass` "/Game/TimeControlSystem/Blueprints/ReplaySystem/BP_CharacterPawn.BP_CharacterPawn_C" (`self.GetTransform` (`|GetArrayItem` _outactors)) "Undefined" "OverrideRootScale" null null))
  (set `self.CharacterPawn` _returnvalue))

(fn `SpawnSpectator`
  (bind _asbp_spectator_pawn (cast `/Game/TimeControlSystem/Blueprints/BP_SpectatorPawn` (`GameplayStatics.GetPlayerPawn` 0)))
  (set `self.SpectatorPawn` _asbp_spectator_pawn))

(fn `SpawnVehicle`
  (bind _outactors (`GameplayStatics.GetAllActorsWithTag` "VehiclePawn"))
  (bind _returnvalue (`|SpawnActorFromClass` "/Game/TimeControlSystem/Blueprints/ReplaySystem/BP_VehiclePawn.BP_VehiclePawn_C" (`self.GetTransform` (`|GetArrayItem` _outactors)) "Undefined" "OverrideRootScale" null null))
  (set `self.VehiclePawn` _returnvalue))

(fn `UserConstructionScript`)