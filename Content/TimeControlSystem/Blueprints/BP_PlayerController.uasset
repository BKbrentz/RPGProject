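; Player controller for the time control system that maps input to time direction, dilation, recording, reverse and replay, and creates a toggleable debug widget.
; Time changes go to BP_GameMode, with hold-driven looping timers on dilation keys, while record and playback messages go to the possessed pawn.
; SwitchPawn possesses the GameMode's spectator, character or vehicle pawn, with multi-click and hold detection on gamepad.
; Debug-draw toggles broadcast to all BPI_TimeControlSystem actors.
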(event `self.ReceiveBeginPlay`
  ;[0 0 0] Event BeginPlay
  (bind _returnvalue (`|CreateWidget` "/Game/TimeControlSystem/Blueprints/Widgets/WB_Debug.WB_Debug_C" self))
  (bind _output_get (set `self.DebugWidget` _returnvalue))
  (`UserWidget.AddToViewport` _output_get 0)
  (`WidgetBlueprintLibrary.SetInputMode_GameOnly` self)
  (bind _asbp_game_mode (cast `/Game/TimeControlSystem/Blueprints/BP_GameMode` (`GameplayStatics.GetGameMode`)))
  (set `self.GameMode` _asbp_game_mode))

(event `InputAction|TimeBackward`
  (params (Key :type "Key Structure"))
  ;[0 0 0] Time Direction Inputs
  (:`Pressed`
    (`/Game/TimeControlSystem/Blueprints/BP_GameMode.SetTimeDirection` (`self.GameMode`) "NewEnumerator1")))

(event `InputAction|TimeForward`
  (params (Key :type "Key Structure"))
  ;[0 0 0] Time Direction Inputs
  (:`Pressed`
    (`/Game/TimeControlSystem/Blueprints/BP_GameMode.SetTimeDirection` (`self.GameMode`) "NewEnumerator0")))

(event `InputAction|DilationIncrease`
  (params (Key :type "Key Structure"))
  ;[0 0 0] Increase / Decrease Time Dilation Inputs
  (:`Pressed`
    (`/Game/TimeControlSystem/Blueprints/BP_GameMode.ModifyTimeDilation` (`self.GameMode`) 0.5)
    (`/Game/TimeControlSystem/Blueprints/BP_Macros.Hold Input` 0.5 :!label _label
      (:`Held`
        (bind _returnvalue (`KismetSystemLibrary.K2_SetTimerDelegate` (`|CreateDelegate` (`self.GameMode`) :!event `IncreaseDilation`) 0.5 true)))
      (:`Cancelled`
        (`KismetSystemLibrary.K2_ClearAndInvalidateTimerHandle` _returnvalue))))
  (:`Released`
    (goto _label :!via `Released`)))

(event `InputAction|DilationDecrease`
  (params (Key :type "Key Structure"))
  ;[0 0 0] Increase / Decrease Time Dilation Inputs
  (:`Pressed`
    (`/Game/TimeControlSystem/Blueprints/BP_GameMode.ModifyTimeDilation` (`self.GameMode`) -0.5)
    (`/Game/TimeControlSystem/Blueprints/BP_Macros.Hold Input` 0.5 :!label _label_2
      (:`Held`
        (bind _returnvalue (`KismetSystemLibrary.K2_SetTimerDelegate` (`|CreateDelegate` (`self.GameMode`) :!event `DecreaseDilation`) 0.5 true)))
      (:`Cancelled`
        (`KismetSystemLibrary.K2_ClearAndInvalidateTimerHandle` _returnvalue))))
  (:`Released`
    (goto _label_2 :!via `Released`)))

(event `InputAction|PawnSpectator`
  (params (Key :type "Key Structure"))
  ;[0 0 0] Switch Pawn Inputs
  (:`Pressed`
    (`self.SwitchPawn` "NewEnumerator0")))

(event `InputAction|PawnCharacter`
  (params (Key :type "Key Structure"))
  ;[0 0 0] Switch Pawn Inputs
  (:`Pressed`
    (`self.SwitchPawn` "NewEnumerator1")))

(event `InputAction|PawnGamepad`
  (params (Key :type "Key Structure"))
  ;[0 0 0] Switch Pawn Inputs
  (:`Pressed`
    (bind _times (`/Game/TimeControlSystem/Blueprints/BP_Macros.Multi-Click Input` 0.2)
      (:`Signle Click`
        (`/Game/TimeControlSystem/Blueprints/BP_Macros.Hold Input` 0.5 :!label _label_3
          (:`Held`
            (`self.SwitchPawn` "NewEnumerator2"))
          (:`Clicked`
            (switch `int` _times
              (:`1`
                (`self.SwitchPawn` "NewEnumerator0"))
              (:`2`
                (`self.SwitchPawn` "NewEnumerator1"))))))))
  (:`Released`
    (goto _label_3 :!via `Released`)))

(event `InputAction|PawnVehicle`
  (params (Key :type "Key Structure"))
  ;[0 0 0] Switch Pawn Inputs
  (:`Pressed`
    (`self.SwitchPawn` "NewEnumerator2")))

(event `InputAction|RecordStart`
  (params (Key :type "Key Structure"))
  ;[0 0 0] Record & Replay & Reverse Inputs
  (:`Pressed`
    (message `/Game/TimeControlSystem/Blueprints/ReplaySystem/BPI_ReplaySystem.StartRecord` (`self.K2_GetPawn`))))

(event `InputAction|RecordStop`
  (params (Key :type "Key Structure"))
  ;[0 0 0] Record & Replay & Reverse Inputs
  (:`Pressed`
    (message `/Game/TimeControlSystem/Blueprints/ReplaySystem/BPI_ReplaySystem.StopRecord` (`self.K2_GetPawn`))))

(event `InputAction|Reverse`
  (params (Key :type "Key Structure"))
  ;[0 0 0] Record & Replay & Reverse Inputs
  (:`Pressed`
    (message `/Game/TimeControlSystem/Blueprints/ReplaySystem/BPI_ReplaySystem.StartReverse` (`self.K2_GetPawn`))))

(event `InputAction|Replay`
  (params (Key :type "Key Structure"))
  ;[0 0 0] Record & Replay & Reverse Inputs
  (:`Pressed`
    (message `/Game/TimeControlSystem/Blueprints/ReplaySystem/BPI_ReplaySystem.StartReplay` (`self.K2_GetPawn`))))

(event `InputAction|ToggleDebugMenu`
  (params (Key :type "Key Structure"))
  ;[0 0 0] Toggle Debug Menu Inputs
  (:`Pressed`
    (`/Game/TimeControlSystem/Blueprints/Widgets/WB_Debug.SwitchDebugMenu` (`self.DebugWidget`))))

(event `InputAction|DrawDebugReversible`
  (params (Key :type "Key Structure"))
  ;[0 0 0] Draw Debug Inputs
  (:`Pressed`
    (bind _isa (`/Engine/EditorBlueprintResources/StandardMacros.FlipFlop`)
      (:`A`
        _)
      (:`B`
        _))
    (bind _outactors (`GameplayStatics.GetAllActorsWithInterface` "/Game/TimeControlSystem/Blueprints/BPI_TimeControlSystem.BPI_TimeControlSystem_C"))
    (message `/Game/TimeControlSystem/Blueprints/BPI_TimeControlSystem.BPI_SetDrawDebugReversible` _outactors _isa)))

(event `InputAction|DrawDebugClock`
  (params (Key :type "Key Structure"))
  ;[0 0 0] Draw Debug Inputs
  (:`Pressed`
    (bind _isa (`/Engine/EditorBlueprintResources/StandardMacros.FlipFlop`)
      (:`A`
        _)
      (:`B`
        _))
    (bind _outactors (`GameplayStatics.GetAllActorsWithInterface` "/Game/TimeControlSystem/Blueprints/BPI_TimeControlSystem.BPI_TimeControlSystem_C"))
    (message `/Game/TimeControlSystem/Blueprints/BPI_TimeControlSystem.BPI_SetDrawDebugClock` _outactors _isa)))

(fn `SwitchPawn`
  (params (PawnType :type "/Game/TimeControlSystem/Blueprints/ReplaySystem/Enum_PawnType Enum" :default "NewEnumerator0"))
  (bind _gamemode (`self.GameMode`))
  (set `self.PawnType` PawnType)
  (`self.Possess` (select `/Game/TimeControlSystem/Blueprints/ReplaySystem/Enum_PawnType` (`self.PawnType`) :`NewEnumerator0` (`/Game/TimeControlSystem/Blueprints/BP_GameMode.SpectatorPawn` _gamemode) :`NewEnumerator1` (`/Game/TimeControlSystem/Blueprints/BP_GameMode.CharacterPawn` _gamemode) :`NewEnumerator2` (`/Game/TimeControlSystem/Blueprints/BP_GameMode.VehiclePawn` _gamemode) :!type "Pawn Object Reference")))

(fn `UserConstructionScript`)