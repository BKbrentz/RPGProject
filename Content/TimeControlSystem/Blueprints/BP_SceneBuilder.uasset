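; BP_SceneBuilder is a configurable static mesh actor in the TimeControlSystem folder, used as a recolorable scene piece.
; Its construction script assigns the chosen mesh, then pushes top and side color pairs, tiling and roughness into the mesh's materials as named parameters.
; All setup happens at construction time; BeginPlay is empty and there is no runtime logic.
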(event `self.ReceiveBeginPlay`)

(fn `UserConstructionScript`
  (`StaticMeshComponent.SetStaticMesh` (`self.StaticMesh`) (`self.Mesh`))
  (`MeshComponent.SetVectorParameterValueOnMaterials` (`self.StaticMesh`) "TopColor_1" (`KismetMathLibrary.Conv_LinearColorToVector` (`self.TopColor 1`)))
  (`MeshComponent.SetVectorParameterValueOnMaterials` (`self.StaticMesh`) "TopColor_2" (`KismetMathLibrary.Conv_LinearColorToVector` (`self.TopColor 2`)))
  (`MeshComponent.SetVectorParameterValueOnMaterials` (`self.StaticMesh`) "SideColor_1" (`KismetMathLibrary.Conv_LinearColorToVector` (`self.SideColor 1`)))
  (`MeshComponent.SetVectorParameterValueOnMaterials` (`self.StaticMesh`) "SideColor_2" (`KismetMathLibrary.Conv_LinearColorToVector` (`self.SideColor 2`)))
  (`MeshComponent.SetScalarParameterValueOnMaterials` (`self.StaticMesh`) "Tiling" (`self.Tiling`))
  (`MeshComponent.SetScalarParameterValueOnMaterials` (`self.StaticMesh`) "Roughness" (`self.Roughness`)))