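; BP_Visualizer is an actor in the time control system folder that displays a scaled, colored static mesh with a configurable text label.
; Its construction script applies the text content, size, color and transform to the TextRender component and sets the mesh scale.
; It also creates a dynamic instance of MI_Visualizer on the mesh to drive its Color parameter.
; The event graph contains no active logic.
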(fn `UserConstructionScript`
  (`TextRenderComponent.K2_SetText` (`self.TextRender`) (`self.TextContent`))
  (`TextRenderComponent.SetWorldSize` (`self.TextRender`) (`self.TextSize`))
  (`TextRenderComponent.SetTextRenderColor` (`self.TextRender`) (`self.TextColor`))
  (`SceneComponent.K2_SetRelativeLocationAndRotation` (`self.TextRender`) (`self.TextLocation`) (`self.TextRotation`) false false)
  (`SceneComponent.SetRelativeScale3D` (`self.StaticMesh`) (`self.Scale`))
  (bind _returnvalue (`PrimitiveComponent.CreateDynamicMaterialInstance` (`self.StaticMesh`) 0 "/Game/TimeControlSystem/Materials/MI_Visualizer.MI_Visualizer" "None"))
  (`MaterialInstanceDynamic.SetVectorParameterValue` _returnvalue "Color" (`self.Color`)))