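; BP_Clock is an analog clock actor that turns hour, minute and second hands to show either system time or a custom time.
; Forward and backward timelines, switched through a time-direction interface, advance or rewind the custom time, committing whole seconds on timeline events.
; Tick maps the displayed time to hand roll, with optional millisecond smoothing and debug text.
; The construction script seeds any custom time and previews the hand positions.
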(event `self.ReceiveBeginPlay`
  (`self.BPI_SetTimeDirection` "NewEnumerator0"))

(event `self.ReceiveTick`
  (params (DeltaSeconds :type "Float (single-precision)"))
  (`self.CalculateRotation`)
  (if (`self.DrawDebug`)
    (`self.DrawDebugString`)))

(event `self.BPI_SetTimeDirection`
  (params (Dir :type "/Game/TimeControlSystem/Blueprints/Enum_TimeDirection Enum" :default "NewEnumerator0"))
  (set `self.TimeDirection` Dir)
  (set `self.LastClockTime` (`self.ClockTime`))
  (switch `/Game/TimeControlSystem/Blueprints/Enum_TimeDirection` (`self.TimeDirection`)
    (:`NewEnumerator0`
      (`TimelineComponent.Stop` (`self.Bwd`))
      (`TimelineComponent.PlayFromStart` (`self.Fwd`)))
    (:`NewEnumerator1`
      (`TimelineComponent.Stop` (`self.Fwd`))
      (`TimelineComponent.PlayFromStart` (`self.Bwd`)))))

(event `self.BPI_SetDrawDebugClock`
  (params (bDrawDebug :type Boolean))
  (set `self.DrawDebug` bDrawDebug))

(fn `CalculateRotation`
  (bind (_hour12 _minute _second _millisecond) (`self.GetTime`))
  (bind _returnvalue (`KismetMathLibrary.Conv_IntToDouble` _second))
  (bind _returnvalue_2 (+ (`KismetMathLibrary.Conv_IntToDouble` _hour12) (/ (`KismetMathLibrary.Conv_IntToDouble` _minute) 60.0)))
  (bind _returnvalue_3 (`KismetMathLibrary.SelectFloat` (+ _returnvalue (/ (`KismetMathLibrary.Conv_IntToDouble` _millisecond) 1000.0)) _returnvalue (`self.UseMillisecond`)))
  (`SceneComponent.K2_SetRelativeRotation` (`self.HourHand`) (`KismetMathLibrary.MakeRotator` (* (`KismetMathLibrary.MapRangeClamped` (`KismetMathLibrary.SelectFloat` (- _returnvalue_2 12.0) _returnvalue_2 (>= _returnvalue_2 12.0)) 0.0 12.0 0.0 360.0) -1.0)) false false)
  (`SceneComponent.K2_SetRelativeRotation` (`self.MinuteHand`) (`KismetMathLibrary.MakeRotator` (* (`KismetMathLibrary.MapRangeClamped` (+ (`KismetMathLibrary.Conv_IntToDouble` _minute) (/ _returnvalue_3 60.0)) 0.0 60.0 0.0 360.0) -1.0)) false false)
  (`SceneComponent.K2_SetRelativeRotation` (`self.SecondHand`) (`KismetMathLibrary.MakeRotator` (* (`KismetMathLibrary.MapRangeClamped` _returnvalue_3 0.0 60.0 0.0 360.0) -1.0)) false false))

(fn `DrawDebugString`
  (bind (_hour12 _minute _second _millisecond) (`self.GetTime`))
  (bind _returnvalue (`KismetStringLibrary.Concat_StrStr` (`KismetStringLibrary.Conv_IntToString` _hour12) ":" (`KismetStringLibrary.Conv_IntToString` _minute) ":" (`KismetStringLibrary.Conv_IntToString` _second)))
  (`KismetSystemLibrary.DrawDebugString` (0.0 0.0 0.0) (`KismetMathLibrary.SelectString` (`KismetStringLibrary.Concat_StrStr` _returnvalue ":" (`KismetStringLibrary.Conv_IntToString` _millisecond)) _returnvalue (`self.UseMillisecond`)) self))

(fn `GetTime`
  (returns (Hour12 :type Integer) (Minute :type Integer) (Second :type Integer) (Millisecond :type Integer))
  (bind _returnvalue (select `bool` (`self.UseCustomTime`) :`false` (`KismetMathLibrary.Now`) :`true` (`self.ClockTime`)))
  (return (`KismetMathLibrary.GetHour12` _returnvalue) (`KismetMathLibrary.GetMinute` _returnvalue) (`KismetMathLibrary.GetSecond` _returnvalue) (`KismetMathLibrary.GetMillisecond` _returnvalue)))

(fn `SetDrawDebug`
  (params (DrawDebug :type Boolean))
  (set `self.DrawDebug` DrawDebug))

(fn `UserConstructionScript`
  (bind (_year _month _day) (`KismetMathLibrary.BreakDateTime` (`KismetMathLibrary.Now`)))
  (`|ExecutionSequence`
    (:`then_0`
      (if (`self.UseCustomTime`)
        (set `self.ClockTime` (`KismetMathLibrary.MakeDateTime` _year _month _day (`self.CustomHour`) (`self.CustomMinute`) (`self.CustomSecond`) (`KismetMathLibrary.SelectInt` (`self.CustomMillisecond`) 0 (`self.UseMillisecond`))))))
    (:`then_1`
      (`self.CalculateRotation`))))