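; Actor component that records a character's movement and plays it back forward or in reverse in a time-control system.
; A looping frame-delta timer samples transform, control rotation, movement axes and jump, then saves them through BP_GameMode.
; Replay and reverse actors spawn with the saved data.
; Playback teleports the capsule while re-feeding input, destroys the AI controller at the end, and Tick can draw the debug path.
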(event `self.ReceiveBeginPlay`
  (bind _asbp_game_mode (cast `/Game/TimeControlSystem/Blueprints/BP_GameMode` (`GameplayStatics.GetGameMode`)))
  (set `self.GameMode` _asbp_game_mode)
  (set `self.ReplayData` (`self.LoadReplayData`)))

(event `self.ReceiveTick`
  (params (DeltaSeconds :type "Float (single-precision)"))
  (if (`self.bDrawDebug`)
    (`self.DrawDebugPath` 5.0)))

(fn `DrawDebugPath`
  (params (DrawLineThickness :type "Float (double-precision)" :default 5.0) (DrawLineColor :type "LinearColor Structure" :default (struct :`R` 1.0 :`G` 1.0 :`B` 1.0 :`A` 1.0)))
  (locals (CurIndex :type Integer) (CurLocation :type "Vector Structure") (LastLocation :type "Vector Structure"))
  (for (_array_element _array_index) (`self.ReplayData`)
    (bind _output_get (set `local.CurIndex` _array_index))
    (bind _transform_location (`KismetMathLibrary.BreakTransform` (break `/Game/TimeControlSystem/Blueprints/ReplaySystem/Struct_ReplayDataCharacter` _array_element)))
    (set `local.CurLocation` _transform_location)
    (`/Engine/EditorBlueprintResources/StandardMacros.CompareInt` _output_get
      (:`>`
        (`KismetSystemLibrary.DrawDebugLine` (`local.LastLocation`) (`local.CurLocation`) (`local.DrawLineColor`) 0.0 (`local.DrawLineThickness`)))
      (:`==`
        _)
      (:`<`
        _))
    (set `local.LastLocation` (`local.CurLocation`))))

(fn `GetAIController`
  (returns (AIController :type "AIController Object Reference"))
  (return (`AIBlueprintHelperLibrary.GetAIController` (`Pawn.GetController` (`self.Character`)))))

(fn `GetCapsuleComponent`
  (returns (CapsuleComponent :type "CapsuleComponent Object Reference"))
  (return (`Character.CapsuleComponent` (`self.Character`))))

(fn `GetCharacterMovement`
  (returns (CharacterMovement :type "CharacterMovementComponent Object Reference"))
  (return (`Character.CharacterMovement` (`self.Character`))))

(fn `GetReplayData`
  (returns (ReplayData :type "/Game/TimeControlSystem/Blueprints/ReplaySystem/Struct_ReplayDataCharacter Structure"))
  (return (`|GetArrayItem` (`self.ReplayData`) (`self.ReplayIndex`))))

(fn `LoadReplayData`
  (returns (ReplayData :type "Array of /Game/TimeControlSystem/Blueprints/ReplaySystem/Struct_ReplayDataCharacter Structure"))
  (bind _savegameobject (`/Game/TimeControlSystem/Blueprints/BP_GameMode.LoadGame` (`self.GameMode`)))
  (`/Engine/EditorBlueprintResources/StandardMacros.IsValid` _savegameobject
    (:`Is Valid`
      (bind _asbp_replay_save_game (cast `/Game/TimeControlSystem/Blueprints/ReplaySystem/BP_ReplaySaveGame` _savegameobject))
      (return (`/Game/TimeControlSystem/Blueprints/ReplaySystem/BP_ReplaySaveGame.CharacterReplayData` _asbp_replay_save_game)))))

(fn `Reocrd`
  (bind _character (`self.Character`))
  (`KismetSystemLibrary.DrawDebugString` (0.0 0.0 0.0) "RECORDING" (`self.Character`) (struct :`R` 1.0 :`G` 0.5 :`A` 1.0))
  (bind (_fwdaxis _rwdaxis) (message `/Game/TimeControlSystem/Blueprints/ReplaySystem/BPI_ReplaySystem.GetCharacterData` _character))
  (`KismetArrayLibrary.Array_Add` (`self.ReplayData`) (make `/Game/TimeControlSystem/Blueprints/ReplaySystem/Struct_ReplayDataCharacter` (`SceneComponent.K2_GetComponentToWorld` (`Character.CapsuleComponent` _character)) (`Pawn.GetControlRotation` _character) _fwdaxis _rwdaxis (`Character.bWasJumping` _character))))

(fn `Replay`
  (bind (_replaydata_transform _replaydata_controlrotation _replaydata_fwd _replaydata_rwd _replaydata_jump) (break `/Game/TimeControlSystem/Blueprints/ReplaySystem/Struct_ReplayDataCharacter` (`self.GetReplayData`)))
  (bind _character (`self.Character`))
  (bind _returnvalue (`KismetMathLibrary.MakeRotator` 0.0 0.0 (.yaw (`Pawn.GetControlRotation` (`self.Character`)))))
  (`|ExecutionSequence`
    (:`then_0`
      (`SceneComponent.K2_SetWorldTransform` (`self.GetCapsuleComponent`) _replaydata_transform false true)
      (`Controller.SetControlRotation` (`self.GetAIController`) _replaydata_controlrotation)
      (`Pawn.AddMovementInput` _character (`KismetMathLibrary.GetForwardVector` _returnvalue) _replaydata_fwd true)
      (`Pawn.AddMovementInput` _character (`KismetMathLibrary.GetRightVector` _returnvalue) _replaydata_rwd true)
      (if _replaydata_jump
        (`Character.Jump` (`self.Character`))))
    (:`then_1`
      (bind _result (`/Engine/EditorBlueprintResources/StandardMacros.IncrementInt` (`self.ReplayIndex`))
        (:`  `
          (if (> _result (`KismetArrayLibrary.Array_LastIndex` (`self.ReplayData`)))
            (`/Engine/EditorBlueprintResources/StandardMacros.DecrementInt` (`self.ReplayIndex`)
              (:`  `
                (`MovementComponent.StopMovementImmediately` (`self.GetCharacterMovement`))
                (`Actor.K2_DestroyActor` (`self.GetAIController`))))))))))

(fn `Reverse`
  (bind (_replaydata_transform _replaydata_controlrotation _replaydata_fwd _replaydata_rwd _replaydata_jump) (break `/Game/TimeControlSystem/Blueprints/ReplaySystem/Struct_ReplayDataCharacter` (`self.GetReplayData`)))
  (bind _character (`self.Character`))
  (bind _returnvalue (`KismetMathLibrary.MakeRotator` 0.0 0.0 (.yaw (`Pawn.GetControlRotation` (`self.Character`)))))
  (`|ExecutionSequence`
    (:`then_0`
      (`SceneComponent.K2_SetWorldTransform` (`self.GetCapsuleComponent`) _replaydata_transform false true)
      (`Controller.SetControlRotation` (`self.GetAIController`) _replaydata_controlrotation)
      (`Pawn.AddMovementInput` _character (`KismetMathLibrary.GetForwardVector` _returnvalue) _replaydata_fwd true)
      (`Pawn.AddMovementInput` _character (`KismetMathLibrary.GetRightVector` _returnvalue) _replaydata_rwd true)
      (if _replaydata_jump
        (`Character.Jump` (`self.Character`))))
    (:`then_1`
      (bind _result (`/Engine/EditorBlueprintResources/StandardMacros.DecrementInt` (`self.ReplayIndex`))
        (:`  `
          (if (< _result 0)
            (`/Engine/EditorBlueprintResources/StandardMacros.IncrementInt` (`self.ReplayIndex`)
              (:`  `
                (`MovementComponent.StopMovementImmediately` (`self.GetCharacterMovement`))
                (`Actor.K2_DestroyActor` (`self.GetAIController`))))))))))

(fn `SetCharacter`
  (params (Character :type "Character Object Reference"))
  (set `self.Character` Character))

(fn `SetReplayData`
  (params (ReplayData :type "Array of /Game/TimeControlSystem/Blueprints/ReplaySystem/Struct_ReplayDataCharacter Structure"))
  (set `self.ReplayData` ReplayData))

(fn `SpawnReplay`
  (bind _replayactor (`self.ReplayActor`))
  (`|ExecutionSequence`
    (:`then_0`
      (`/Engine/EditorBlueprintResources/StandardMacros.IsValid` _replayactor
        (:`Is Valid`
          (`Actor.K2_DestroyActor` _replayactor))))
    (:`then_1`
      (bind _returnvalue (`|SpawnActorFromClass` "/Game/TimeControlSystem/Blueprints/ReplaySystem/BP_CharacterReplay.BP_CharacterReplay_C" (`Actor.GetTransform` (`self.Character`)) "AlwaysSpawn" "OverrideRootScale" null (`self.LoadReplayData`) null))
      (set `self.ReplayActor` _returnvalue))))

(fn `SpawnReverse`
  (bind _reverseactor (`self.ReverseActor`))
  (`|ExecutionSequence`
    (:`then_0`
      (`/Engine/EditorBlueprintResources/StandardMacros.IsValid` _reverseactor
        (:`Is Valid`
          (`Actor.K2_DestroyActor` _reverseactor))))
    (:`then_1`
      (bind _returnvalue (`|SpawnActorFromClass` "/Game/TimeControlSystem/Blueprints/ReplaySystem/BP_CharacterReverse.BP_CharacterReverse_C" (`Actor.GetTransform` (`self.Character`)) "AlwaysSpawn" "OverrideRootScale" null (`self.LoadReplayData`) null))
      (set `self.ReverseActor` _returnvalue))))

(fn `StartRecord`
  (`KismetArrayLibrary.Array_Clear` (`self.ReplayData`))
  (bind _returnvalue (`KismetSystemLibrary.K2_SetTimerDelegate` (`|CreateDelegate` :!event `Reocrd`) (`GameplayStatics.GetWorldDeltaSeconds`) true))
  (set `self.RecordTimer` _returnvalue))

(fn `StartReplay`
  (bind _returnvalue (`KismetSystemLibrary.K2_SetTimerDelegate` (`|CreateDelegate` :!event `Replay`) (`GameplayStatics.GetWorldDeltaSeconds`) true))
  (set `self.ReplayTimer` _returnvalue))

(fn `StartReverse`
  (set `self.ReplayIndex` (`KismetArrayLibrary.Array_LastIndex` (`self.ReplayData`)))
  (bind _returnvalue (`KismetSystemLibrary.K2_SetTimerDelegate` (`|CreateDelegate` :!event `Reverse`) (`GameplayStatics.GetWorldDeltaSeconds`) true))
  (set `self.ReverseTimer` _returnvalue))

(fn `StopRecord`
  (returns (bSaved :type Boolean))
  (`KismetSystemLibrary.K2_ClearAndInvalidateTimerHandle` (`self.RecordTimer`))
  (bind _savegameobject (`/Game/TimeControlSystem/Blueprints/BP_GameMode.LoadGame` (`self.GameMode`)))
  (bind (_asbp_replay_save_game _bsuccess) (cast `/Game/TimeControlSystem/Blueprints/ReplaySystem/BP_ReplaySaveGame` _savegameobject :!pure true))
  (bind _returnvalue (`/Game/TimeControlSystem/Blueprints/BP_GameMode.SaveGame` (`self.GameMode`) (`self.ReplayData`) (select `bool` _bsuccess :`false` (`|MakeArray`) :`true` (`/Game/TimeControlSystem/Blueprints/ReplaySystem/BP_ReplaySaveGame.VehicleReplayData` _asbp_replay_save_game))))
  (return _returnvalue))