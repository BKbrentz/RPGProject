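; Vehicle component that records a vehicle's motion and plays it back forward or in reverse, as part of a time control system.
; Looping timers at frame delta sample mesh transform, steering, throttle and handbrake, or reapply them by teleporting the mesh and feeding movement inputs.
; Stopping a recording saves through BP_GameMode, preserving character replay data.
; Saved data seeds spawned replay and reverse vehicles, and the path can be debug-drawn.
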(event `self.ReceiveBeginPlay`
  (bind _asbp_game_mode (cast `/Game/TimeControlSystem/Blueprints/BP_GameMode` (`GameplayStatics.GetGameMode`)))
  (set `self.GameMode` _asbp_game_mode)
  (set `self.ReplayData` (`self.LoadReplayData`)))

(event `self.ReceiveTick`
  (params (DeltaSeconds :type "Float (single-precision)"))
  (if (`self.bDrawDebug`)
    (`self.DrawDebugPath` 5.0)))

(fn `DrawDebugPath`
  (params (DrawLineThickness :type "Float (double-precision)" :default 5.0) (DrawLineColor :type "LinearColor Structure" :default (struct :`R` 1.0 :`G` 1.0 :`B` 1.0 :`A` 1.0)))
  (locals (CurIndex :type Integer) (CurLocation :type "Vector Structure") (LastLocation :type "Vector Structure"))
  (for (_array_element _array_index) (`self.ReplayData`)
    (bind _output_get (set `local.CurIndex` _array_index))
    (bind _transform_location (`KismetMathLibrary.BreakTransform` (break `/Game/TimeControlSystem/Blueprints/ReplaySystem/Struct_ReplayDataVehicle` _array_element)))
    (set `local.CurLocation` _transform_location)
    (`/Engine/EditorBlueprintResources/StandardMacros.CompareInt` _output_get
      (:`>`
        (`KismetSystemLibrary.DrawDebugLine` (`local.LastLocation`) (`local.CurLocation`) (`local.DrawLineColor`) 0.0 (`local.DrawLineThickness`)))
      (:`==`
        _)
      (:`<`
        _))
    (set `local.LastLocation` (`local.CurLocation`))))

(fn `GetAIController`
  (returns (AIController :type "AIController Object Reference"))
  (return (`AIBlueprintHelperLibrary.GetAIController` (`Pawn.GetController` (`self.Vehicle`)))))

(fn `GetMesh`
  (returns (Mesh :type "SkeletalMeshComponent Object Reference"))
  (return (`WheeledVehicle.Mesh` (`self.Vehicle`))))

(fn `GetReplayData`
  (returns (ReplayData :type "/Game/TimeControlSystem/Blueprints/ReplaySystem/Struct_ReplayDataVehicle Structure"))
  (return (`|GetArrayItem` (`self.ReplayData`) (`self.ReplayIndex`))))

(fn `GetVehicleMovement`
  (returns (VehicleMovement :type "WheeledVehicleMovementComponent Object Reference"))
  (return (`WheeledVehicle.VehicleMovement` (`self.Vehicle`))))

(fn `LoadReplayData`
  (returns (ReplayData :type "Array of /Game/TimeControlSystem/Blueprints/ReplaySystem/Struct_ReplayDataVehicle Structure"))
  (bind _savegameobject (`/Game/TimeControlSystem/Blueprints/BP_GameMode.LoadGame` (`self.GameMode`)))
  (`/Engine/EditorBlueprintResources/StandardMacros.IsValid` _savegameobject
    (:`Is Valid`
      (bind _asbp_replay_save_game (cast `/Game/TimeControlSystem/Blueprints/ReplaySystem/BP_ReplaySaveGame` _savegameobject))
      (return (`/Game/TimeControlSystem/Blueprints/ReplaySystem/BP_ReplaySaveGame.VehicleReplayData` _asbp_replay_save_game)))))

(fn `Reocrd`
  (`KismetSystemLibrary.DrawDebugString` (0.0 0.0 0.0) "RECORDING" (`self.Vehicle`) (struct :`R` 1.0 :`G` 0.5 :`A` 1.0))
  (bind (_steering _throttle _handbrake) (message `/Game/TimeControlSystem/Blueprints/ReplaySystem/BPI_ReplaySystem.GetVehicleData` (`self.Vehicle`)))
  (`KismetArrayLibrary.Array_Add` (`self.ReplayData`) (make `/Game/TimeControlSystem/Blueprints/ReplaySystem/Struct_ReplayDataVehicle` (`SceneComponent.K2_GetComponentToWorld` (`self.GetMesh`)) _steering _throttle _handbrake)))

(fn `Replay`
  (bind _vehiclemovement (`self.GetVehicleMovement`))
  (bind (_replaydata_transform _replaydata_steering _replaydata_throttle _replaydata_handbrake) (break `/Game/TimeControlSystem/Blueprints/ReplaySystem/Struct_ReplayDataVehicle` (`self.GetReplayData`)))
  (`|ExecutionSequence`
    (:`then_0`
      (`SceneComponent.K2_SetWorldTransform` (`self.GetMesh`) _replaydata_transform false true)
      (`WheeledVehicleMovementComponent.SetSteeringInput` _vehiclemovement _replaydata_steering)
      (`WheeledVehicleMovementComponent.SetThrottleInput` _vehiclemovement _replaydata_throttle)
      (`WheeledVehicleMovementComponent.SetHandbrakeInput` _vehiclemovement _replaydata_handbrake)
      (`KismetSystemLibrary.DrawDebugString` (0.0 0.0 0.0) "REPLAYING" (`self.Vehicle`) (struct :`R` 1.0 :`A` 1.0)))
    (:`then_1`
      (bind _result (`/Engine/EditorBlueprintResources/StandardMacros.IncrementInt` (`self.ReplayIndex`))
        (:`  `
          (if (> _result (`KismetArrayLibrary.Array_LastIndex` (`self.ReplayData`)))
            (`/Engine/EditorBlueprintResources/StandardMacros.DecrementInt` (`self.ReplayIndex`)
              (:`  `
                (`MovementComponent.StopMovementImmediately` (`self.GetVehicleMovement`))))))))))

(fn `Reverse`
  (bind _vehiclemovement (`self.GetVehicleMovement`))
  (bind (_replaydata_transform _replaydata_steering _replaydata_throttle _replaydata_handbrake) (break `/Game/TimeControlSystem/Blueprints/ReplaySystem/Struct_ReplayDataVehicle` (`self.GetReplayData`)))
  (`|ExecutionSequence`
    (:`then_0`
      (`SceneComponent.K2_SetWorldTransform` (`self.GetMesh`) _replaydata_transform false true)
      (`WheeledVehicleMovementComponent.SetSteeringInput` _vehiclemovement _replaydata_steering)
      (`WheeledVehicleMovementComponent.SetThrottleInput` _vehiclemovement _replaydata_throttle)
      (`WheeledVehicleMovementComponent.SetHandbrakeInput` _vehiclemovement _replaydata_handbrake)
      (`KismetSystemLibrary.DrawDebugString` (0.0 0.0 0.0) "REVERSING" (`self.Vehicle`) (struct :`G` 1.0 :`A` 1.0)))
    (:`then_1`
      (bind _result (`/Engine/EditorBlueprintResources/StandardMacros.DecrementInt` (`self.ReplayIndex`))
        (:`  `
          (if (< _result 0)
            (`/Engine/EditorBlueprintResources/StandardMacros.IncrementInt` (`self.ReplayIndex`)
              (:`  `
                (`MovementComponent.StopMovementImmediately` (`self.GetVehicleMovement`))))))))))

(fn `SetReplayData`
  (params (ReplayData :type "Array of /Game/TimeControlSystem/Blueprints/ReplaySystem/Struct_ReplayDataVehicle Structure"))
  (set `self.ReplayData` ReplayData))

(fn `SetVehicle`
  (params (Vehicle :type "WheeledVehicle Object Reference"))
  (set `self.Vehicle` Vehicle))

(fn `SpawnReplay`
  (bind _replayactor (`self.ReplayActor`))
  (`|ExecutionSequence`
    (:`then_0`
      (`/Engine/EditorBlueprintResources/StandardMacros.IsValid` _replayactor
        (:`Is Valid`
          (`Actor.K2_DestroyActor` _replayactor))))
    (:`then_1`
      (bind _returnvalue (`|SpawnActorFromClass` "/Game/TimeControlSystem/Blueprints/ReplaySystem/BP_VehicleReplay.BP_VehicleReplay_C" (`Actor.GetTransform` (`self.Vehicle`)) "AlwaysSpawn" "OverrideRootScale" null (`self.LoadReplayData`) null))
      (set `self.ReplayActor` _returnvalue))))

(fn `SpawnReverse`
  (bind _reverseactor (`self.ReverseActor`))
  (`|ExecutionSequence`
    (:`then_0`
      (`/Engine/EditorBlueprintResources/StandardMacros.IsValid` _reverseactor
        (:`Is Valid`
          (`Actor.K2_DestroyActor` _reverseactor))))
    (:`then_1`
      (bind _returnvalue (`|SpawnActorFromClass` "/Game/TimeControlSystem/Blueprints/ReplaySystem/BP_VehicleReverse.BP_VehicleReverse_C" (`Actor.GetTransform` (`self.Vehicle`)) "AlwaysSpawn" "OverrideRootScale" null (`self.LoadReplayData`) null))
      (set `self.ReverseActor` _returnvalue))))

(fn `StartRecord`
  (`KismetArrayLibrary.Array_Clear` (`self.ReplayData`))
  (bind _returnvalue (`KismetSystemLibrary.K2_SetTimerDelegate` (`|CreateDelegate` :!event `Reocrd`) (`GameplayStatics.GetWorldDeltaSeconds`) true))
  (set `self.RecordTimer` _returnvalue))

(fn `StartReplay`
  (bind _returnvalue (`KismetSystemLibrary.K2_SetTimerDelegate` (`|CreateDelegate` :!event `Replay`) (`GameplayStatics.GetWorldDeltaSeconds`) true))
  (set `self.ReplayTimer` _returnvalue))

(fn `StartReverse`
  (set `self.ReplayIndex` (`KismetArrayLibrary.Array_LastIndex` (`self.ReplayData`)))
  (bind _returnvalue (`KismetSystemLibrary.K2_SetTimerDelegate` (`|CreateDelegate` :!event `Reverse`) (`GameplayStatics.GetWorldDeltaSeconds`) true))
  (set `self.ReverseTimer` _returnvalue))

(fn `StopRecord`
  (returns (bSaved :type Boolean))
  (`KismetSystemLibrary.K2_ClearAndInvalidateTimerHandle` (`self.RecordTimer`))
  (bind _savegameobject (`/Game/TimeControlSystem/Blueprints/BP_GameMode.LoadGame` (`self.GameMode`)))
  (bind (_asbp_replay_save_game _bsuccess) (cast `/Game/TimeControlSystem/Blueprints/ReplaySystem/BP_ReplaySaveGame` _savegameobject :!pure true))
  (bind _returnvalue (`/Game/TimeControlSystem/Blueprints/BP_GameMode.SaveGame` (`self.GameMode`) (select `bool` _bsuccess :`false` (`|MakeArray`) :`true` (`/Game/TimeControlSystem/Blueprints/ReplaySystem/BP_ReplaySaveGame.CharacterReplayData` _asbp_replay_save_game)) (`self.ReplayData`)))
  (return _returnvalue))