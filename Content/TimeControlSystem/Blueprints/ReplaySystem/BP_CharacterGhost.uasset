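; BP_CharacterGhost is a short-lived ghost actor that shows a frozen pose of a character.
; Its construction script applies a custom lifespan, offset, mesh and one override material across all slots of a poseable mesh.
; On BeginPlay it copies the pose from a given skeletal mesh component once, or destroys itself if that component is invalid.
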(event `self.ReceiveBeginPlay`
  (`self.ComponentToCopy`
    (:`then`
      (`PoseableMeshComponent.CopyPoseFromSkeletalComponent` (`self.PoseableMesh`) (`self.ComponentToCopy`)))
    (:`else`
      (`self.K2_DestroyActor`))))

(fn `UserConstructionScript`
  (`self.SetLifeSpan` (`self.CustomLifeSpan`))
  (`SceneComponent.K2_SetRelativeTransform` (`self.PoseableMesh`) (`self.CustomOffset`) false false)
  (`SkinnedMeshComponent.SetSkinnedAssetAndUpdate` (`self.PoseableMesh`) (`self.CustomMesh`) true)
  (for _index (range 1 (+ (`PrimitiveComponent.GetNumMaterials` (`self.PoseableMesh`)) 1))
    (`PrimitiveComponent.SetMaterial` (`self.PoseableMesh`) (- _index 1) (`self.CustomMaterial`))))