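; BP_CharacterReplay is a replay character that plays back recorded data in the time control system.
; Its construction script registers the actor as the character of its CharacterReplaySystem.
; On BeginPlay, it hands ReplayData to that system, teleports its capsule to the first recorded transform and starts the replay.
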(event `self.ReceiveBeginPlay`
  (`/Game/TimeControlSystem/Blueprints/ReplaySystem/ACBP_ReplaySystemCharacter.SetReplayData` (`self.CharacterReplaySystem`) (`self.ReplayData`))
  (`SceneComponent.K2_SetWorldTransform` (`self.CapsuleComponent`) (`.Transform_2_0FF334DD4FC78F68A4BDE086B66E8FA3` (break `/Game/TimeControlSystem/Blueprints/ReplaySystem/Struct_ReplayDataCharacter` (`|GetArrayItem` (`self.ReplayData`)))) false true)
  (`/Game/TimeControlSystem/Blueprints/ReplaySystem/ACBP_ReplaySystemCharacter.StartReplay` (`self.CharacterReplaySystem`)))

(fn `UserConstructionScript`
  (`/Game/TimeControlSystem/Blueprints/ReplaySystem/ACBP_ReplaySystemCharacter.SetCharacter` (`self.CharacterReplaySystem`) self))