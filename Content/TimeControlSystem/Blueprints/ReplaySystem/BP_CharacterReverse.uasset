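; BP_CharacterReverse is a character in the time control replay system that plays recorded replay data backwards.
; The construction script registers the character with its CharacterReplaySystem.
; On BeginPlay it passes its ReplayData to that system, teleports the capsule to the last recorded transform, then starts the reverse playback.
; The playback logic itself lives in CharacterReplaySystem.
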(event `self.ReceiveBeginPlay`
  (bind _replaydata (`self.ReplayData`))
  (`/Game/TimeControlSystem/Blueprints/ReplaySystem/ACBP_ReplaySystemCharacter.SetReplayData` (`self.CharacterReplaySystem`) (`self.ReplayData`))
  (`SceneComponent.K2_SetWorldTransform` (`self.CapsuleComponent`) (`.Transform_2_0FF334DD4FC78F68A4BDE086B66E8FA3` (break `/Game/TimeControlSystem/Blueprints/ReplaySystem/Struct_ReplayDataCharacter` (`|GetArrayItem` _replaydata (`KismetArrayLibrary.Array_LastIndex` _replaydata)))) false true)
  (`/Game/TimeControlSystem/Blueprints/ReplaySystem/ACBP_ReplaySystemCharacter.StartReverse` (`self.CharacterReplaySystem`)))

(fn `UserConstructionScript`
  (`/Game/TimeControlSystem/Blueprints/ReplaySystem/ACBP_ReplaySystemCharacter.SetCharacter` (`self.CharacterReplaySystem`) self))