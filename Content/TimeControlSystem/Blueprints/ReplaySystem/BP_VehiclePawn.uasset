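; Drivable vehicle pawn that can record its run and spawn replay or reverse playback through the VehicleReplaySystem.
; Axis and handbrake inputs drive VehicleMovement and are cached for GetVehicleData, while GetCharacterData returns zeros.
; Interface events forward record, replay and reverse calls to the replay system, which is bound to this pawn at construction.
; It caches its AI controller on possession and hands control back to it when a player controller unpossesses.
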(event `InputAxis|ViewY`
  (params (AxisValue :type "Float (single-precision)"))
  ;[0 0 0] View Inputs
  (`self.AddControllerPitchInput` AxisValue))

(event `InputAxis|ViewX`
  (params (AxisValue :type "Float (single-precision)"))
  ;[0 0 0] View Inputs
  (`self.AddControllerYawInput` AxisValue))

(event `InputAxis|MoveX`
  (params (AxisValue :type "Float (single-precision)"))
  ;[0 0 0] Steering Inputs
  (bind _output_get (set `self.Streering` AxisValue))
  (`WheeledVehicleMovementComponent.SetSteeringInput` (`self.VehicleMovement`) _output_get))

(event `InputAxis|MoveY`
  (params (AxisValue :type "Float (single-precision)"))
  ;[0 0 0] Throttle Inputs
  (bind _output_get (set `self.Throttle` AxisValue))
  (`WheeledVehicleMovementComponent.SetThrottleInput` (`self.VehicleMovement`) _output_get))

(event `InputAction|Handbrake`
  (params (Key :type "Key Structure"))
  (bind _vehiclemovement (`self.VehicleMovement`))
  ;[0 0 0] Handbrake Inputs
  (:`Pressed`
    (bind _output_get (set `self.Handbrake` true))
    (`WheeledVehicleMovementComponent.SetHandbrakeInput` _vehiclemovement _output_get))
  (:`Released`
    (bind _output_get_2 (set `self.Handbrake` false))
    (`WheeledVehicleMovementComponent.SetHandbrakeInput` _vehiclemovement _output_get_2)))

(event `self.ReceivePossessed`
  (params (NewController :type "Controller Object Reference"))
  (bind _asaicontroller (cast `AIController` NewController))
  (set `self.AIController` _asaicontroller))

(event `self.ReceiveUnpossessed`
  (params (OldController :type "Controller Object Reference"))
  (if (`Controller.IsPlayerController` OldController)
    (`Controller.Possess` (`self.AIController`) self)))

(event `/Game/TimeControlSystem/Blueprints/ReplaySystem/BPI_ReplaySystem.StartRecord`
  (`/Game/TimeControlSystem/Blueprints/ReplaySystem/ACBP_ReplaySystemVehicle.StartRecord` (`self.VehicleReplaySystem`)))

(event `/Game/TimeControlSystem/Blueprints/ReplaySystem/BPI_ReplaySystem.StopRecord`
  (bind _bsaved (`/Game/TimeControlSystem/Blueprints/ReplaySystem/ACBP_ReplaySystemVehicle.StopRecord` (`self.VehicleReplaySystem`)))
  (if _bsaved
    (`KismetSystemLibrary.PrintString` "Game has been saved." true false (struct :`G` 1.0 :`A` 1.0))
    (else
      (`KismetSystemLibrary.PrintString` "Failed to save game." true false (struct :`G` 1.0 :`A` 1.0)))))

(event `/Game/TimeControlSystem/Blueprints/ReplaySystem/BPI_ReplaySystem.StartReplay`
  (`/Game/TimeControlSystem/Blueprints/ReplaySystem/ACBP_ReplaySystemVehicle.SpawnReplay` (`self.VehicleReplaySystem`)))

(event `/Game/TimeControlSystem/Blueprints/ReplaySystem/BPI_ReplaySystem.StartReverse`
  (`/Game/TimeControlSystem/Blueprints/ReplaySystem/ACBP_ReplaySystemVehicle.SpawnReverse` (`self.VehicleReplaySystem`)))

(fn `GetCharacterData`
  (returns (FwdAxis :type "Float (double-precision)") (RwdAxis :type "Float (double-precision)"))
  (return 0.0 0.0))

(fn `GetVehicleData`
  (returns (Steering :type "Float (double-precision)") (Throttle :type "Float (double-precision)") (Handbrake :type Boolean))
  (return (`self.Streering`) (`self.Throttle`) (`self.Handbrake`)))

(fn `UserConstructionScript`
  (`/Game/TimeControlSystem/Blueprints/ReplaySystem/ACBP_ReplaySystemVehicle.SetVehicle` (`self.VehicleReplaySystem`) self))