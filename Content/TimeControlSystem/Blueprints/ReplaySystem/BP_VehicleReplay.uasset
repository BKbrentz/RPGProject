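; BP_VehicleReplay is a vehicle actor that plays back recorded replay data through its VehicleReplaySystem.
; The construction script registers the actor as that system's vehicle.
; On BeginPlay it passes ReplayData to the system, teleports the mesh to the first recorded transform and starts playback immediately.
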(event `self.ReceiveBeginPlay`
  (`/Game/TimeControlSystem/Blueprints/ReplaySystem/ACBP_ReplaySystemVehicle.SetReplayData` (`self.VehicleReplaySystem`) (`self.ReplayData`))
  (`SceneComponent.K2_SetWorldTransform` (`self.Mesh`) (`.Transform_2_0FF334DD4FC78F68A4BDE086B66E8FA3` (break `/Game/TimeControlSystem/Blueprints/ReplaySystem/Struct_ReplayDataVehicle` (`|GetArrayItem` (`self.ReplayData`)))) false true)
  (`/Game/TimeControlSystem/Blueprints/ReplaySystem/ACBP_ReplaySystemVehicle.StartReplay` (`self.VehicleReplaySystem`)))

(fn `UserConstructionScript`
  (`/Game/TimeControlSystem/Blueprints/ReplaySystem/ACBP_ReplaySystemVehicle.SetVehicle` (`self.VehicleReplaySystem`) self))