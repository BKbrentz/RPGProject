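; Vehicle actor that plays recorded replay data in reverse, as part of the time control system.
; The construction script registers the actor as the vehicle of its VehicleReplaySystem.
; On BeginPlay it passes ReplayData to that system, teleports the mesh to the last recorded transform and starts reverse playback.
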(event `self.ReceiveBeginPlay`
  (bind _replaydata (`self.ReplayData`))
  (`/Game/TimeControlSystem/Blueprints/ReplaySystem/ACBP_ReplaySystemVehicle.SetReplayData` (`self.VehicleReplaySystem`) (`self.ReplayData`))
  (`SceneComponent.K2_SetWorldTransform` (`self.Mesh`) (`.Transform_2_0FF334DD4FC78F68A4BDE086B66E8FA3` (break `/Game/TimeControlSystem/Blueprints/ReplaySystem/Struct_ReplayDataVehicle` (`|GetArrayItem` _replaydata (`KismetArrayLibrary.Array_LastIndex` _replaydata)))) false true)
  (`/Game/TimeControlSystem/Blueprints/ReplaySystem/ACBP_ReplaySystemVehicle.StartReverse` (`self.VehicleReplaySystem`)))

(fn `UserConstructionScript`
  (`/Game/TimeControlSystem/Blueprints/ReplaySystem/ACBP_ReplaySystemVehicle.SetVehicle` (`self.VehicleReplaySystem`) self))