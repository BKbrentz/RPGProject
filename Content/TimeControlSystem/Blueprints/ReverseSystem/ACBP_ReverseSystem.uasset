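; Actor component that records a component's motion and plays it back in reverse for time rewinding.
; A looping timer appends world transform and velocity to arrays while time runs forward.
; Switching to backward runs a timer scaled by ReverseSpeed that applies and pops those samples, optionally destroying the owner when history runs out.
; Both directions fire callbacks, and a debug timer can draw the path and state.
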(event `self.ReceiveBeginPlay`
  (bind _returnvalue (`self.GetOwner`))
  (set `self.CurTransform` (`Actor.GetTransform` _returnvalue))
  (set `self.CurVelocity` (`Actor.GetVelocity` _returnvalue))
  (`self.DirectionSwitcher`))

(fn `DirectionSwitcher`
  (switch `/Game/TimeControlSystem/Blueprints/Enum_TimeDirection` (`self.CurTimeDir`)
    (:`NewEnumerator0`
      (`KismetSystemLibrary.K2_ClearAndInvalidateTimerHandle` (`self.TimerBwd`))
      (bind _returnvalue (`KismetSystemLibrary.K2_SetTimerDelegate` (`|CreateDelegate` :!event `TimeForward`) (`self.Duration`) true))
      (set `self.TimerFwd` _returnvalue))
    (:`NewEnumerator1`
      (`KismetSystemLibrary.K2_ClearAndInvalidateTimerHandle` (`self.TimerFwd`))
      (bind _returnvalue_2 (`KismetSystemLibrary.K2_SetTimerDelegate` (`|CreateDelegate` :!event `TimeBackward`) (/ (`self.Duration`) (`self.ReverseSpeed`)) true))
      (set `self.TimerBwd` _returnvalue_2))))

(fn `DrawDebug`
  (locals (CurIndex :type Integer) (CurLocation :type "Vector Structure" :default (0.0 0.0 0.0)) (DrawDuration :type "Float (double-precision)" :default 0.1) (DrawPoints :type Boolean :default false) (DrawPointColor :type "LinearColor Structure" :default (struct :`R` 1.0 :`G` 1.0 :`B` 1.0 :`A` 1.0)) (DrawPointSize :type "Float (double-precision)" :default 10.0) (DrawLineColor :type "LinearColor Structure" :default (struct :`R` 0.7 :`G` 0.7 :`B` 0.7 :`A` 1.0)) (DrawLineThickness :type "Float (double-precision)" :default 2.0) (DrawLocation :type Boolean :default false) (LastLocation :type "Vector Structure" :default (0.0 0.0 0.0)) (DrawState :type Boolean :default true))
  (bind _drawduration (`local.DrawDuration`))
  (bind _component (`self.Component`))
  (bind _origin (`KismetSystemLibrary.GetComponentBounds` (`self.Component`)))
  (bind (_origin_2 _boxextent _sphereradius) (`KismetSystemLibrary.GetComponentBounds` (`self.Component`)))
  (`|ExecutionSequence`
    (:`then_0`
      (for (_array_element _array_index) (`self.Transform`)
        (bind _output_get (set `local.CurIndex` _array_index))
        (set `local.CurLocation` (.location _array_element))
        (`/Engine/EditorBlueprintResources/StandardMacros.CompareInt` _output_get
          (:`>`
            (`KismetSystemLibrary.DrawDebugLine` (`local.LastLocation`) (`local.CurLocation`) (`local.DrawLineColor`) (`local.DrawDuration`) (`local.DrawLineThickness`)))
          (:`==`
            _)
          (:`<`
            _))
        (set `local.LastLocation` (`local.CurLocation`))
        (if (`local.DrawPoints`)
          (`KismetSystemLibrary.DrawDebugPoint` (`local.CurLocation`) (`local.DrawPointSize`) (`local.DrawPointColor`) (`local.DrawDuration`)))))
    (:`then_1`
      (if (`local.DrawLocation`)
        (`KismetSystemLibrary.DrawDebugString` (+ _origin_2 (`KismetMathLibrary.MakeVector` 0.0 0.0 _sphereradius)) (`KismetStringLibrary.Concat_StrStr` "Location:   " (`KismetStringLibrary.Conv_VectorToString` (.location (`SceneComponent.K2_GetComponentToWorld` _component))) " \n" "Velocity:   " (`KismetStringLibrary.Conv_VectorToString` (`SceneComponent.GetComponentVelocity` _component)) " \n" "NumPoints:   " (`KismetStringLibrary.Conv_IntToString` (`KismetArrayLibrary.Array_Length` (`self.Transform`)))) null (struct :`R` 1.0 :`G` 1.0 :`B` 1.0 :`A` 1.0) (`local.DrawDuration`))))
    (:`then_2`
      (if (`local.DrawState`)
        (`/Engine/EditorBlueprintResources/StandardMacros.CompareFloat` (`KismetMathLibrary.VSize` (`SceneComponent.GetComponentVelocity` (`self.Component`)))
          (:`>`
            (`KismetSystemLibrary.DrawDebugString` _origin "MOVING" null (struct :`G` 1.0 :`A` 1.0) _drawduration))
          (:`==`
            (`KismetSystemLibrary.DrawDebugString` _origin "STATIC" null (struct :`R` 1.0 :`G` 1.0 :`A` 1.0) _drawduration :!label _label))
          (:`<`
            (goto _label)))))))

(fn `SetComponent`
  (params (Component :type "PrimitiveComponent Object Reference"))
  (set `self.Component` Component))

(fn `SetShouldDestroy`
  (params (bDestroy :type Boolean))
  (set `self.bShouldDestroy` bDestroy))

(fn `SetShowDebug`
  (params (bShowDebug :type Boolean))
  (bind _output_get (set `self.bShowDebug` bShowDebug))
  (if _output_get
    (bind _returnvalue (`KismetSystemLibrary.K2_SetTimer` self "DrawDebug" 0.1 true))
    (set `self.TimerDebug` _returnvalue)
    (else
      (`KismetSystemLibrary.K2_ClearAndInvalidateTimerHandle` (`self.TimerDebug`)))))

(fn `SetTimeDirection`
  (params (OldDir :type "/Game/TimeControlSystem/Blueprints/Enum_TimeDirection Enum" :default "NewEnumerator0"))
  (set `self.CurTimeDir` OldDir)
  (`self.DirectionSwitcher`))

(fn `TimeBackward`
  (bind _velocity (`self.Velocity`))
  (bind _transform (`self.Transform`))
  (bind _returnvalue (`KismetArrayLibrary.Array_LastIndex` _velocity))
  (bind _returnvalue_2 (`KismetArrayLibrary.Array_LastIndex` _transform))
  (`self.Bwd`)
  (`|ExecutionSequence`
    (:`then_0`
      (`SceneComponent.K2_SetWorldTransform` (`self.Component`) (`|GetArrayItem` _transform _returnvalue_2) false false)
      (`/Engine/EditorBlueprintResources/StandardMacros.CompareInt` _returnvalue_2
        (:`>`
          (`KismetArrayLibrary.Array_Remove` _transform _returnvalue_2))))
    (:`then_1`
      (`PrimitiveComponent.SetPhysicsLinearVelocity` (`self.Component`) (`|GetArrayItem` _velocity _returnvalue) false "None")
      (`/Engine/EditorBlueprintResources/StandardMacros.CompareInt` _returnvalue
        (:`>`
          (`KismetArrayLibrary.Array_Remove` (`self.Velocity`) _returnvalue))))
    (:`then_2`
      (if (and (`self.bShouldDestroy`) (or (<= (`KismetArrayLibrary.Array_Length` (`self.Transform`)) 1) (<= (`KismetArrayLibrary.Array_Length` (`self.Velocity`)) 1)))
        (`Actor.K2_DestroyActor` (`self.GetOwner`))))))

(fn `TimeForward`
  (`self.Fwd`)
  (`|ExecutionSequence`
    (:`then_0`
      (bind _output_get (set `self.CurTransform` (`SceneComponent.K2_GetComponentToWorld` (`self.Component`))))
      (`KismetArrayLibrary.Array_Add` (`self.Transform`) _output_get))
    (:`then_1`
      (bind _output_get_2 (set `self.CurVelocity` (`SceneComponent.GetComponentVelocity` (`self.Component`))))
      (`KismetArrayLibrary.Array_Add` (`self.Velocity`) _output_get_2))))