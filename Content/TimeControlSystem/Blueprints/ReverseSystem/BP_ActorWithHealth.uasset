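; Actor with health and a widget healthbar in the TimeControlSystem's ReverseSystem folder, with no rewind logic of its own.
; AnyDamage subtracts from current health, refills it to max at zero or below, then updates the WB_Healthbar.
; Tick shows the bar only while the player camera is closer than HealthbarVisibleDist.
; The construction script clamps current health between zero and max; ReceiveDamage is an empty stub.
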(event `self.ReceiveBeginPlay`
  (bind _aswb_healthbar (cast `/Game/TimeControlSystem/Blueprints/Widgets/WB_Healthbar` (`WidgetComponent.GetUserWidgetObject` (`self.Widget`))))
  (bind _output_get (set `self.WB_Healthbar` _aswb_healthbar))
  (`/Game/TimeControlSystem/Blueprints/Widgets/WB_Healthbar.SetHealthValue` _output_get (`self.HealthCur`) (`self.HealthMax`)))

(event `self.ReceiveAnyDamage`
  (params (Damage :type "Float (single-precision)") (DamageType :type "DamageType Object Reference") (InstigatedBy :type "Controller Object Reference") (DamageCauser :type "Actor Object Reference"))
  (set `self.Damage` Damage)
  (set `self.HealthCur` (- (`self.HealthCur`) (`self.Damage`)))
  (`|ExecutionSequence`
    (:`then_0`
      (`/Engine/EditorBlueprintResources/StandardMacros.CompareFloat` (`self.HealthCur`)
        (:`==`
          _)
        (:`<`
          _))
      (set `self.HealthCur` (`self.HealthMax`)))
    (:`then_1`
      (`/Game/TimeControlSystem/Blueprints/Widgets/WB_Healthbar.SetHealthValue` (`self.WB_Healthbar`) (`self.HealthCur`) (`self.HealthMax`)))))

(event `self.ReceiveTick`
  (params (DeltaSeconds :type "Float (single-precision)"))
  (bind _widget (`self.Widget`))
  (`/Engine/EditorBlueprintResources/StandardMacros.CompareFloat` (`self.HealthbarVisibleDist`) (`self.GetDistanceTo` (`GameplayStatics.GetPlayerCameraManager` 0) self)
    (:`>`
      (`SceneComponent.SetVisibility` _widget true true))
    (:`==`
      (`SceneComponent.SetVisibility` _widget false true :!label _label))
    (:`<`
      (goto _label))))

(fn `ReceiveDamage`)

(fn `UserConstructionScript`
  (bind _healthcur (`self.HealthCur`))
  (`|ExecutionSequence`
    (:`then_1`
      (`/Engine/EditorBlueprintResources/StandardMacros.CompareFloat` _healthcur (`self.HealthMax`)
        (:`>`
          (set `self.HealthCur` (`self.HealthMax`)))
        (:`<`
          (`/Engine/EditorBlueprintResources/StandardMacros.CompareFloat` _healthcur
            (:`<`
              (set `self.HealthCur` 0.0))))))))