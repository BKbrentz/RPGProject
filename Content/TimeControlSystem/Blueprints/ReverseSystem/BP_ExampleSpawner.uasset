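; Example spawner for the time-reversal system that creates self-destroying BP_ReversibleActors at random points inside a configurable box.
; SetTimeDirection, called on BeginPlay and through an interface, swaps looping forward and backward timers.
; Forward ticks unbind tracked actors' OnDestroyed and spawn; backward ticks bind it to prune the Actors map, which is debug-drawn each frame.
; Arrow-based impulse launching, scale-in timeline and map registration are disconnected, so live spawns go untracked.
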(event `self.ReceiveBeginPlay`
  (if (`self.bEnabled`)
    (`self.SetTimeDirection` "NewEnumerator0")))

(event `self.ReceiveTick`
  (params (DeltaSeconds :type "Float (single-precision)"))
  (`self.DrawDebugString`))

(event `SpawnActors`
  (bind _randompoint (`self.RandomPoint`))
  (bind (_origin _boxextent) (`KismetSystemLibrary.GetComponentBounds` (`self.BoxCollision`)))
  (`|ExecutionSequence`
    (:`then_0`
      (bind _keys (`BlueprintMapLibrary.Map_Keys` (`self.Actors`)))
      (for _array_element _keys
        (`/Engine/EditorBlueprintResources/StandardMacros.IsValid` _array_element
          (:`Is Valid`
            (remove `self.OnDestroyed` _array_element (`|CreateDelegate` :!event `Destroyed`))))))
    (:`then_1`
      (set `self.RandomPoint` (`KismetMathLibrary.RandomPointInBoundingBox` _origin _boxextent))
      (`KismetSystemLibrary.DrawDebugPoint` _randompoint 10.0 (struct :`A` 1.0) 5.0)
      (bind _returnvalue (`|SpawnActorFromClass` "/Game/TimeControlSystem/Blueprints/ReverseSystem/BP_ReversibleActor.BP_ReversibleActor_C" (`KismetMathLibrary.MakeTransform` _randompoint (`KismetMathLibrary.RandomRotator` true) (0.5 0.5 0.5)) "Undefined" "OverrideRootScale" null null))
      (bind _output_get (set `self.TempActor` _returnvalue))
      (`/Game/TimeControlSystem/Blueprints/ReverseSystem/ACBP_ReverseSystem.SetShouldDestroy` (`/Game/TimeControlSystem/Blueprints/ReverseSystem/BP_ReversibleActor.ReverseSystem` _output_get) true))))

(event `ReverseActors`
  (bind _keys (`BlueprintMapLibrary.Map_Keys` (`self.Actors`)))
  (for _array_element _keys
    (`/Engine/EditorBlueprintResources/StandardMacros.IsValid` _array_element
      (:`Is Valid`
        (add `self.OnDestroyed` _array_element (`|CreateDelegate` :!event `Destroyed`))))))

(event `Destroyed` :!signature `self.OnDestroyed`
  (params (DestroyedActor :type "Actor Object Reference"))
  (bind _asbp_reversible_actor (cast `/Game/TimeControlSystem/Blueprints/ReverseSystem/BP_ReversibleActor` DestroyedActor))
  (`BlueprintMapLibrary.Map_Remove` (`self.Actors`) _asbp_reversible_actor))

(event `/Game/TimeControlSystem/Blueprints/BPI_TimeControlSystem.BPI_SetTimeDirection`
  (params (Dir :type "/Game/TimeControlSystem/Blueprints/Enum_TimeDirection Enum" :default "NewEnumerator0"))
  (`self.SetTimeDirection` Dir))

(fn `DrawDebugString`
  (locals (Array :type String))
  (bind _keys (`BlueprintMapLibrary.Map_Keys` (`self.Actors`)))
  (for _array_element _keys
    (set `local.Array` (`KismetStringLibrary.Concat_StrStr` (`local.Array`) " \n" (`KismetSystemLibrary.GetDisplayName` _array_element))))
  (`KismetSystemLibrary.DrawDebugString` (0.0 0.0 0.0) (`local.Array`) self))

(fn `SetTimeDirection`
  (params (TimeDirection :type "/Game/TimeControlSystem/Blueprints/Enum_TimeDirection Enum" :default "NewEnumerator0"))
  (bind _output_get (set `self.TimeDirection` TimeDirection))
  (switch `/Game/TimeControlSystem/Blueprints/Enum_TimeDirection` _output_get
    (:`NewEnumerator0`
      (`KismetSystemLibrary.K2_ClearAndInvalidateTimerHandle` (`self.BwdTimer`))
      (bind _returnvalue (`KismetSystemLibrary.K2_SetTimerDelegate` (`|CreateDelegate` :!event `SpawnActors`) (`self.SpawnDuration`) true))
      (set `self.FwdTimer` _returnvalue))
    (:`NewEnumerator1`
      (`KismetSystemLibrary.K2_ClearAndInvalidateTimerHandle` (`self.FwdTimer`))
      (bind _returnvalue_2 (`KismetSystemLibrary.K2_SetTimerDelegate` (`|CreateDelegate` :!event `ReverseActors`) (`self.ReverseDuration`) true))
      (set `self.BwdTimer` _returnvalue_2))))

(fn `UserConstructionScript`
  (`SceneComponent.K2_SetRelativeTransform` (`self.BoxCollision`) (`self.VolumeTransform`) false false)
  (`BoxComponent.SetBoxExtent` (`self.BoxCollision`) (`self.VolumeExtent`) true))