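; Projectile actor that deals damage on hit and undoes that damage when time runs backward.
; A TimeControlSystem component is set up on the collision sphere, whose collision is disabled during reversal.
; Hits are stored by the component's latest recorded transform index; the backward callback looks them up, applies negative damage and removes them.
; Alternative trace-based approaches remain as unconnected, never-run nodes.
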(event `self.SphereCollision.OnComponentHit`
  (params (HitComponent :type "PrimitiveComponent Object Reference") (OtherActor :type "Actor Object Reference") (OtherComp :type "PrimitiveComponent Object Reference") (NormalImpulse :type "Vector Structure") (Hit :type "HitResult Structure (by ref)"))
  (`GameplayStatics.ApplyDamage` OtherActor (`self.HitDamage`))
  (`KismetSystemLibrary.DrawDebugString` (`self.K2_GetActorLocation`) "HIT" null (struct :`R` 1.0 :`A` 1.0) 0.1)
  (`BlueprintMapLibrary.Map_Add` (`self.Hits`) (`KismetArrayLibrary.Array_LastIndex` (`/Game/TimeControlSystem/Blueprints/ReverseSystem/ACBP_ReverseSystem.Transform` (`self.TimeControlSystem`))) Hit))

(event `/Game/TimeControlSystem/Blueprints/BPI_TimeControlSystem.BPI_SetTimeDirection`
  (params (Dir :type "/Game/TimeControlSystem/Blueprints/Enum_TimeDirection Enum" :default "NewEnumerator0"))
  (`/Game/TimeControlSystem/Blueprints/ReverseSystem/ACBP_ReverseSystem.SetTimeDirection` (`self.TimeControlSystem`) Dir)
  (switch `/Game/TimeControlSystem/Blueprints/Enum_TimeDirection` Dir
    (:`NewEnumerator0`
      (`PrimitiveComponent.SetCollisionEnabled` (`self.SphereCollision`) "QueryAndPhysics"))
    (:`NewEnumerator1`
      (`PrimitiveComponent.SetCollisionEnabled` (`self.SphereCollision`) "NoCollision"))))

(event `BwdTrace`
  (bind (_value _returnvalue) (`BlueprintMapLibrary.Map_Find` (`self.Hits`) (`KismetArrayLibrary.Array_LastIndex` (`/Game/TimeControlSystem/Blueprints/ReverseSystem/ACBP_ReverseSystem.Transform` (`self.TimeControlSystem`)))))
  (if _returnvalue
    (`GameplayStatics.ApplyDamage` (`.HitActor` (`GameplayStatics.BreakHitResult` _value)) (* (`self.HitDamage`) -1.0))
    (`BlueprintMapLibrary.Map_Remove` (`self.Hits`) (`KismetArrayLibrary.Array_LastIndex` (`/Game/TimeControlSystem/Blueprints/ReverseSystem/ACBP_ReverseSystem.Transform` (`self.TimeControlSystem`))))))

(fn `UserConstructionScript`
  (`/Game/TimeControlSystem/Blueprints/ReverseSystem/ACBP_ReverseSystem.SetComponent` (`self.TimeControlSystem`) (`self.SphereCollision`))
  (add `/Game/TimeControlSystem/Blueprints/ReverseSystem/ACBP_ReverseSystem.Bwd` (`self.TimeControlSystem`) (`|CreateDelegate` :!event `BwdTrace`)))