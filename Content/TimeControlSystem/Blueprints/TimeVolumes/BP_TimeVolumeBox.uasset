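; BP_TimeVolumeBox is a box-shaped time volume in the time control system.
; Box collision begin and end overlap events pass the other actor to ActorEnter and ActorLeave, which handle the response outside this graph.
; The construction script runs the parent's, sizes the collision from VolumeExtent, scales the visual mesh to match, and applies main and edge colors as material parameters.
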(event `self.BoxCollision.OnComponentBeginOverlap`
  (params (OverlappedComponent :type "PrimitiveComponent Object Reference") (OtherActor :type "Actor Object Reference") (OtherComp :type "PrimitiveComponent Object Reference") (OtherBodyIndex :type Integer) (bFromSweep :type Boolean) (SweepResult :type "HitResult Structure (by ref)"))
  (`self.ActorEnter` OtherActor))

(event `self.BoxCollision.OnComponentEndOverlap`
  (params (OverlappedComponent :type "PrimitiveComponent Object Reference") (OtherActor :type "Actor Object Reference") (OtherComp :type "PrimitiveComponent Object Reference") (OtherBodyIndex :type Integer))
  (`self.ActorLeave` OtherActor))

(fn `UserConstructionScript`
  (bind _volumeextent (`self.VolumeExtent`))
  (bind _boxmesh (`self.BoxMesh`))
  (`parent.UserConstructionScript`)
  (`BoxComponent.SetBoxExtent` (`self.BoxCollision`) _volumeextent true)
  (`SceneComponent.SetRelativeScale3D` _boxmesh (* (* _volumeextent 2.0) 0.01))
  (`MeshComponent.SetVectorParameterValueOnMaterials` _boxmesh "MainColor" (`KismetMathLibrary.Conv_LinearColorToVector` (`self.VolumeMainColor`)))
  (`MeshComponent.SetVectorParameterValueOnMaterials` _boxmesh "EdgeColor" (`KismetMathLibrary.Conv_LinearColorToVector` (`self.VolumeEdgeColor`))))