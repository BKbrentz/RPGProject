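; BP_TimeVolumeSphere is a spherical time volume in the time control system.
; Begin and end overlaps on its sphere collision are forwarded to ActorEnter and ActorLeave.
; After running the parent construction script, it sizes the collision from VolumeRadius, scales the visible sphere mesh to match, and passes main and edge colors to the mesh materials.
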(event `self.SphereCollision.OnComponentBeginOverlap`
  (params (OverlappedComponent :type "PrimitiveComponent Object Reference") (OtherActor :type "Actor Object Reference") (OtherComp :type "PrimitiveComponent Object Reference") (OtherBodyIndex :type Integer) (bFromSweep :type Boolean) (SweepResult :type "HitResult Structure (by ref)"))
  (`self.ActorEnter` OtherActor))

(event `self.SphereCollision.OnComponentEndOverlap`
  (params (OverlappedComponent :type "PrimitiveComponent Object Reference") (OtherActor :type "Actor Object Reference") (OtherComp :type "PrimitiveComponent Object Reference") (OtherBodyIndex :type Integer))
  (`self.ActorLeave` OtherActor))

(fn `UserConstructionScript`
  (bind _spheremesh (`self.SphereMesh`))
  (bind _volumeradius (`self.VolumeRadius`))
  (`parent.UserConstructionScript`)
  (`SphereComponent.SetSphereRadius` (`self.SphereCollision`) _volumeradius true)
  (`SceneComponent.SetRelativeScale3D` _spheremesh (`KismetMathLibrary.Conv_DoubleToVector` (* _volumeradius 2.0 0.01)))
  (`MeshComponent.SetVectorParameterValueOnMaterials` _spheremesh "MainColor" (`KismetMathLibrary.Conv_LinearColorToVector` (`self.VolumeMainColor`)))
  (`MeshComponent.SetVectorParameterValueOnMaterials` _spheremesh "EdgeColor" (`KismetMathLibrary.Conv_LinearColorToVector` (`self.VolumeEdgeColor`))))